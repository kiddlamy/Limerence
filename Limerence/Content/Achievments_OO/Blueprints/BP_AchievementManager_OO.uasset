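; Achievement manager that tracks, persists and announces unlocked achievements.
; On BeginPlay it loads or creates the AchievementSave slot, then rebuilds matching AchievmentsMap entries with Unlocked set to true.
; UnlockAchievement adds a new ID to the save, writes it immediately and shows an unlock tile widget with the achievement's name if the map contains it.
; Unlocking leaves the map's Unlocked flag untouched until saved unlocks are next loaded.
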(event `self.ReceiveBeginPlay`
  (bind _returnvalue (`GameplayStatics.DoesSaveGameExist` "AchievementSave"))
  (`KismetSystemLibrary.PrintString` "Exist?")
  (if _returnvalue
    (bind _returnvalue_2 (`GameplayStatics.LoadGameFromSlot` "AchievementSave"))
    (`KismetSystemLibrary.PrintString` "Loading")
    (bind _asbp_achievement_save (cast `/Game/Achievments_OO/Blueprints/BP_AchievementSave` _returnvalue_2))
    (set `self.AchievementSave` _asbp_achievement_save)
    (else
      (bind _returnvalue_3 (`GameplayStatics.CreateSaveGameObject` "/Game/Achievments_OO/Blueprints/BP_AchievementSave.BP_AchievementSave_C"))
      (`KismetSystemLibrary.PrintString` "Creating")
      (bind _output_get (set `self.AchievementSave` _returnvalue_3))
      (`GameplayStatics.SaveGameToSlot` _output_get "AchievementSave")
      (`KismetSystemLibrary.PrintString` "Saving")))
  (`self.LoadUnlockedAchievements`))

(fn `LoadUnlockedAchievements`
  (bind _achievmentsmap (`self.AchievmentsMap`))
  (for _array_element (`/Game/Achievments_OO/Blueprints/BP_AchievementSave.UnlockedAchievements` (`self.AchievementSave`))
    (bind (_value _returnvalue) (`BlueprintMapLibrary.Map_Find` _achievmentsmap _array_element))
    (if _returnvalue
      (bind (_id _name _description) (break `/Game/Achievments_OO/Blueprints/ST_Achievements_OO` _value))
      (`BlueprintMapLibrary.Map_Add` _achievmentsmap _array_element (make `/Game/Achievments_OO/Blueprints/ST_Achievements_OO` _id _name _description true)))))

(fn `UnlockAchievement`
  (params (ID :type Name))
  (bind _achievementsave (`self.AchievementSave`))
  (bind (_value _returnvalue) (`BlueprintMapLibrary.Map_Find` (`self.AchievmentsMap`) ID))
  (bind _unlockedachievements (`/Game/Achievments_OO/Blueprints/BP_AchievementSave.UnlockedAchievements` _achievementsave))
  ; Check for achievements and save if locked then show unlock notification - Lamy
  (`/Engine/EditorBlueprintResources/StandardMacros.IsValid` _achievementsave
    (:`Is Valid`
      (`KismetSystemLibrary.PrintString` "AchievementSave VALID")
      (if (not (`KismetArrayLibrary.Array_Contains` _unlockedachievements ID))
        (`KismetArrayLibrary.Array_Add` _unlockedachievements ID)
        (`GameplayStatics.SaveGameToSlot` (`self.AchievementSave`) "AchievementSave")
        (if _returnvalue
          (bind _returnvalue_2 (`|CreateWidget` "/Game/Achievments_OO/Widgets/WB_AchievmentUnlockTile_OO.WB_AchievmentUnlockTile_OO_C" null (`.Name_14_A7B365D34995CB9B44DE11A1FFC18D8F` (break `/Game/Achievments_OO/Blueprints/ST_Achievements_OO` _value))))
          (`UserWidget.AddToViewport` _returnvalue_2 0))))
    (:`Is Not Valid`
      (`KismetSystemLibrary.PrintString` "AchievementSave NULL"))))