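; BP_SpiritLetter_FB_Child is a readable letter pickup that shows only while the player's spirit camera is active, checked every Tick.
; Its custom event uses a FlipFlop to open a letter widget filled from ItemData, locking look and move input and hiding the mesh, then reverse this.
; Sphere overlap toggles a widget, and OnCollected hides the actor.
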(event `CustomEvent`
  (bind _returnvalue (`GameplayStatics.GetPlayerController` 0))
  (bind _letter (`self.Letter`))
  (`/Engine/EditorBlueprintResources/StandardMacros.FlipFlop`
    (:`A`
      (`GameplayStatics.PlaySoundAtLocation` "/Game/Free_Sounds_Pack/wav/Book_Page_1-2.Book_Page_1-2" (`SceneComponent.K2_GetComponentLocation` (`self.Letter`)) (struct) 1.0 1.0 0.0 null null null null)
      (bind _returnvalue_2 (`|CreateWidget` "/Game/ProgrammerMechanics/LetterSystem_FB/WBP_LetterWidget_FB.WBP_LetterWidget_FB_C"))
      (set `/Game/ProgrammerMechanics/LetterSystem_FB/WBP_LetterWidget_FB.Letter Content` (`.LetterContent_17_57E00CFE4CD7D9616F26DB839FA9A5D2` (break `/Game/ProgrammerMechanics/Inventory_FB/ST_InventoryItemStruct_FB` (`self.ItemData`))) _returnvalue_2)
      (`UserWidget.AddToViewport` _returnvalue_2 0)
      (`Controller.SetIgnoreLookInput` _returnvalue true)
      (`Controller.SetIgnoreMoveInput` _returnvalue true)
      (`SceneComponent.SetVisibility` _letter false false))
    (:`B`
      (`/Game/ProgrammerMechanics/LetterSystem_FB/WBP_LetterWidget_FB.Put Down Letter` _returnvalue_2)
      (`Controller.SetIgnoreLookInput` _returnvalue false)
      (`Controller.SetIgnoreMoveInput` _returnvalue false)
      (`SceneComponent.SetVisibility` _letter true false))))

(event `/Game/ProgrammerMechanics/Inventory_FB/BPI_InventoryInteract_FB.OnCollected`
  (`self.SetActorHiddenInGame` true))

(event `self.Sphere.OnComponentBeginOverlap`
  (params (OverlappedComponent :type "PrimitiveComponent Object Reference") (OtherActor :type "Actor Object Reference") (OtherComp :type "PrimitiveComponent Object Reference") (OtherBodyIndex :type Integer) (bFromSweep :type Boolean) (SweepResult :type "HitResult Structure (by ref)"))
  (`SceneComponent.SetVisibility` (`self.Widget`) true false))

(event `self.ReceiveTick`
  (params (DeltaSeconds :type "Float (single-precision)"))
  ; Visibility when spirit cam is active - Lamy
  (bind _asbp_first_person_character (cast `/Game/FirstPerson/Blueprints/BP_FirstPersonCharacter` (`GameplayStatics.GetPlayerCharacter` (`KismetMathLibrary.FTrunc` DeltaSeconds))))
  (if (`/Game/FirstPerson/Blueprints/BP_FirstPersonCharacter.SpiritCameraActive` _asbp_first_person_character)
    (`SceneComponent.SetHiddenInGame` (`self.Letter`) false false)
    (else
      (`SceneComponent.SetHiddenInGame` (`self.Letter`) true false))))

(event `self.Sphere.OnComponentEndOverlap`
  (params (OverlappedComponent :type "PrimitiveComponent Object Reference") (OtherActor :type "Actor Object Reference") (OtherComp :type "PrimitiveComponent Object Reference") (OtherBodyIndex :type Integer))
  (`SceneComponent.SetVisibility` (`self.Widget`) false false))

(fn `UserConstructionScript`
  (`parent.UserConstructionScript`))