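; Inventory component that stores an actor's items, each with an ID, name, icon and letter content, in the InventoryItems array.
; AddItem searches by ItemID and appends only new items; a match is rewritten with its own existing fields, so duplicates neither stack nor update.
; RemoveItem deletes the first entry with a matching ItemID.
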(fn `AddItem`
  (params (Item :type "/Game/ProgrammerMechanics/Inventory_FB/ST_InventoryItemStruct_FB Structure"))
  (bind _inventoryitems (`self.InventoryItems`))
  (for (_array_element _array_index) _inventoryitems
    (bind (_itemname _itemid _itemicon _lettercontent) (break `/Game/ProgrammerMechanics/Inventory_FB/ST_InventoryItemStruct_FB` _array_element))
    (if (== (`.ItemID_8_A356955F4624F582642963AB16B2E8C9` (break `/Game/ProgrammerMechanics/Inventory_FB/ST_InventoryItemStruct_FB` Item)) _itemid)
      (`KismetArrayLibrary.Array_Set` _inventoryitems _array_index (make `/Game/ProgrammerMechanics/Inventory_FB/ST_InventoryItemStruct_FB` _itemname _itemid _itemicon _lettercontent) true)
      (return)))
  (`KismetArrayLibrary.Array_Add` _inventoryitems Item))

(fn `RemoveItem`
  (params (ItemID :type Integer))
  (bind _inventoryitems (`self.InventoryItems`))
  (for (_array_element _array_index) _inventoryitems
    (if (== ItemID (`.ItemID_8_A356955F4624F582642963AB16B2E8C9` (break `/Game/ProgrammerMechanics/Inventory_FB/ST_InventoryItemStruct_FB` _array_element)))
      (`KismetArrayLibrary.Array_Remove` _inventoryitems _array_index)
      (return))))