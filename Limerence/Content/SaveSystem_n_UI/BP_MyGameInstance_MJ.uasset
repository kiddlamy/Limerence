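; Game instance that owns the save game for the project, exposing save and load of game data and player location.
; On Init it loads the existing SaveGameData_MJ from the save slot, or creates a fresh object if none exists, and caches it.
; Save functions update the cached object and write it to the slot immediately, while load functions read straight from that cached copy.
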(event `self.ReceiveInit`
  (bind _returnvalue (`GameplayStatics.DoesSaveGameExist` (`self.Save Slot Name`)))
  (if _returnvalue
    (bind _returnvalue_2 (`GameplayStatics.LoadGameFromSlot` (`self.Save Slot Name`)))
    (bind _assave_game_data_mj (cast `/Game/SaveSystem_n_UI/SaveGameData_MJ` _returnvalue_2))
    (set `self.Save Game Data` _assave_game_data_mj)
    (else
      (bind _returnvalue_3 (`GameplayStatics.CreateSaveGameObject` "/Game/SaveSystem_n_UI/SaveGameData_MJ.SaveGameData_MJ_C"))
      (set `self.Save Game Data` _returnvalue_3))))

(fn `Load Player Location`
  (returns (NewParam :type "Vector Structure"))
  (return (`/Game/SaveSystem_n_UI/SaveGameData_MJ.Player Location` (`self.Save Game Data`))))

(fn `LoadGameData`
  (returns (`Game Data` :type "/Game/SaveSystem_n_UI/GameData_MJ Structure"))
  (return (`/Game/SaveSystem_n_UI/SaveGameData_MJ.Game Data` (`self.Save Game Data`))))

(fn `Save Player Location`
  (params (`Player Position` :type "Vector Structure"))
  (bind _save_game_data (`self.Save Game Data`))
  (set `/Game/SaveSystem_n_UI/SaveGameData_MJ.Player Location` `Player Position` _save_game_data)
  (`GameplayStatics.SaveGameToSlot` _save_game_data (`self.Save Slot Name`)))

(fn `SaveGameData`
  (params (`Game Data` :type "/Game/SaveSystem_n_UI/GameData_MJ Structure"))
  (bind _save_game_data (`self.Save Game Data`))
  (set `/Game/SaveSystem_n_UI/SaveGameData_MJ.Game Data` `Game Data` _save_game_data)
  (`GameplayStatics.SaveGameToSlot` _save_game_data (`self.Save Slot Name`)))