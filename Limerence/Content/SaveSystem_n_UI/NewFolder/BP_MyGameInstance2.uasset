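; BP_MyGameInstance2 is a game instance that handles a save slot for the player's location.
; On Init it loads an existing SaveGameData2; otherwise it creates one but sets the stored reference to None.
; SavePlayerLocation writes a zero vector, ignoring its PlayerPosition input, then saves to the slot.
; LoadPlayerLocation returns the stored location, and a broken cast remains unconnected.
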(event `self.ReceiveInit`
  (bind _returnvalue (`GameplayStatics.DoesSaveGameExist` (`self.Save Slot Name`)))
  (if _returnvalue
    (bind _returnvalue_2 (`GameplayStatics.LoadGameFromSlot` (`self.Save Slot Name`)))
    (bind _assave_game_data_2 (cast `/Game/SaveSystem_n_UI/NewFolder/SaveGameData2` _returnvalue_2))
    (set `self.Save Game Data` _assave_game_data_2)
    (else
      (`GameplayStatics.CreateSaveGameObject` "/Game/SaveSystem_n_UI/NewFolder/SaveGameData2.SaveGameData2_C")
      (set `self.Save Game Data` null))))

(fn `Load Player Location`
  (returns (NewParam :type "Vector Structure"))
  (return (`/Game/SaveSystem_n_UI/NewFolder/SaveGameData2.Player Location` (`self.Save Game Data`))))

(fn `Save Player Location`
  (params (`Player Position` :type "Vector Structure"))
  (bind _save_game_data (`self.Save Game Data`))
  (set `/Game/SaveSystem_n_UI/NewFolder/SaveGameData2.Player Location` (0.0 0.0 0.0) _save_game_data)
  (`GameplayStatics.SaveGameToSlot` _save_game_data (`self.Save Slot Name`)))