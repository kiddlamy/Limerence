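; BP_MyGameMode is a game mode Blueprint that obtains the save data object for the game.
; A custom event reads the save slot name from BP_MyGameInstance_MJ, then loads the existing SaveGameData_MJ from that slot or creates a new one.
; The result is stored in its SaveGameData variable; nothing here calls the event or writes the save to disk.
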(event `CustomEvent`
  (bind _asbp_my_game_instance_mj (cast `/Game/SaveSystem_n_UI/BP_MyGameInstance_MJ` (`GameplayStatics.GetGameInstance`)))
  (bind _output_get (set `self.Save File Name` (`/Game/SaveSystem_n_UI/BP_MyGameInstance_MJ.Save File Name` _asbp_my_game_instance_mj)))
  (bind _returnvalue (`GameplayStatics.DoesSaveGameExist` _output_get))
  (if _returnvalue
    (bind _returnvalue_2 (`GameplayStatics.LoadGameFromSlot` (`self.Save File Name`)))
    (bind _assave_game_data_mj (cast `/Game/SaveSystem_n_UI/SaveGameData_MJ` _returnvalue_2))
    (set `self.Save Game Data` _assave_game_data_mj)
    (else
      (bind _returnvalue_3 (`GameplayStatics.CreateSaveGameObject` "/Game/SaveSystem_n_UI/SaveGameData_MJ.SaveGameData_MJ_C"))
      (set `self.Save Game Data` _returnvalue_3))))

(fn `UserConstructionScript`)